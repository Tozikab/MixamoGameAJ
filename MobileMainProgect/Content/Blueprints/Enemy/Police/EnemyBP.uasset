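; EnemyBP is an armed police enemy that fires tracers and takes damage.
; On BeginPlay it attaches an MP_15 to the Weapon socket and binds the player's destruction to delayed self-removal.
; Shooting spawns a short-lived TracerBP from an arrow and sets a Fire flag.
; DamageEnemy shows a hit widget and lowers health; death shows a second widget, disables capsule collision, plays an animation, then removes enemy and weapon.
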(event Custom|DamageEnemy
  (params (Damage :type Float%20%28single-precision%29))
  ;[1 1 1] Health
  (bind _returnvalue (Game|ConstructObjectfromClass "/Game/HUD/HitEnemy.HitEnemy_C" (Variables|Default|GetCharacter)))
  (UserInterface|Viewport|AddtoViewport _returnvalue 0)
  (bind _output_get (Variables|Default|SetCorrentHealth (- (Variables|Default|GetCorrentHealth) Damage)))
  (if (<= _output_get 0.0)
    (CallFunction|Death)))

(event Custom|StopShooting
  (Variables|Default|SetFire false))

(event Custom|Shooting
  (Variables|Default|SetFire true)
  (bind _returnvalue (Game|SpawnActorfromClass "/Game/Blueprints/Effect/TracerBP.TracerBP_C" (Transformation|GetWorldTransform (Variables|Default|GetArrow1)) "Undefined" 0 0))
  (Actor|SetLifeSpan _returnvalue 1.0))

(event Custom|Death
  (bind _returnvalue (Game|ConstructObjectfromClass "/Game/HUD/HitEnemy_2.HitEnemy_2_C" (Variables|Default|GetCharacter)))
  (UserInterface|Viewport|AddtoViewport _returnvalue 0)
  (Collision|SetCollisionEnabled (Variables|Collision|GetCapsuleComponent) "NoCollision")
  (Components|Animation|PlayAnimation (Variables|Character|GetMesh) "/Game/Blueprints/Enemy/Police/Animation/Death_From_Front_Headshot.Death_From_Front_Headshot" false)
  (Utilities|FlowControl|Delay 2e+01)
  (Actor|DestroyActor (Variables|Default|GetMP15))
  (Actor|DestroyActor))

(event Custom|DeathDelay
  (params (DestroyedActor :type Actor%20Object%20Reference))
  (Utilities|FlowControl|Delay 2.0)
  (Actor|DestroyActor)
  (Actor|DestroyActor (stale EventBeginPlay _output_get)))

(event EventBeginPlay
  (bind _returnvalue (Game|GetPlayerCharacter 0))
  (bind _mesh (Variables|Character|GetMesh))
  (Utilities|FlowControl|Sequence
    (:then_0
      (bind _returnvalue_2 (Game|SpawnActorfromClass "/Game/Assets/Weapon/Mp15/MP_15.MP_15_C" (Transformation|GetWorldTransform _mesh) "Undefined" 0 0))
      (bind _output_get (Variables|Default|SetMP15 _returnvalue_2))
      (Transformation|AttachComponentToComponent _output_get _mesh "Weapon" "SnapToTarget" "SnapToTarget" "SnapToTarget" true))
    (:then_1
      (bind _ascharacter_bp (Utilities|Casting|CastToCharacter_BP _returnvalue))
      (Variables|Default|SetCharacter _ascharacter_bp)
      (Game|BindEventtoOnDestroyed _returnvalue (delegate Custom|DeathDelay)))))

(event EventTick
  (params (DeltaSeconds :type Float%20%28single-precision%29)))

(fn ConstructionScript)

(fn OnRepDamage
  (if (Variables|Default|GetDamage)
    (Variables|Default|SetDamage false)))