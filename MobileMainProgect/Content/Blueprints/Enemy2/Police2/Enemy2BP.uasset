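; Enemy2BP is a police enemy character that carries a baton (Dubinka), attacks with a hit montage and can be killed.
; On BeginPlay it caches the player character, then spawns the baton and attaches it to a mesh socket.
; DamageEnemy shows a hit widget and lowers health, adding a second widget and calling Death at zero.
; Death updates AI blackboard state, disables capsule collision, plays a death animation, then destroys baton and enemy after a delay.
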(event Custom|DamageEnemy
  (params (Damage :type Float%20%28single-precision%29))
  (bind _returnvalue (Game|ConstructObjectfromClass "/Game/HUD/HitEnemy.HitEnemy_C" (Variables|Default|GetCharacterBP)))
  (UserInterface|Viewport|AddtoViewport _returnvalue 0)
  (bind _output_get (Variables|Default|SetCorrentHealth (- (Variables|Default|GetCorrentHealth) Damage)))
  (if (<= _output_get 0.0)
    (AI|Components|Blackboard|SetValueasBool (AI|GetBlackboard 0) (Utilities|Name|MakeLiteralName "CharacterIsDead") true)
    (bind _returnvalue_2 (Game|ConstructObjectfromClass "/Game/HUD/HitEnemy_2.HitEnemy_2_C" (Variables|Default|GetCharacterBP)))
    (UserInterface|Viewport|AddtoViewport _returnvalue_2 0)
    (CallFunction|Death)))

(event Custom|Attack
  (Animation|Montage|PlayMontage (Variables|Character|GetMesh) "/Game/Blueprints/Enemy2/Police2/Animation/Hit.Hit"))

(event Custom|Death
  (bind _output_get (Variables|Default|SetCurrentState "NewEnumerator2"))
  (AI|Components|Blackboard|SetValueasEnum (AI|GetBlackboard 0) (Utilities|Name|MakeLiteralName "AiState") _output_get)
  (Collision|SetCollisionEnabled (Variables|Collision|GetCapsuleComponent) "NoCollision")
  (Components|Animation|PlayAnimation (Variables|Character|GetMesh) "/Game/Blueprints/Enemy2/Police2/Animation/Standing_React_Death_Left.Standing_React_Death_Left" false)
  (Utilities|FlowControl|Delay 2e+01)
  (Actor|DestroyActor (Variables|Default|GetDubinka))
  (Actor|DestroyActor))

(event EventBeginPlay
  (bind _mesh (Variables|Character|GetMesh))
  (bind _ascharacter_bp (Utilities|Casting|CastToCharacter_BP (Game|GetPlayerCharacter 0)))
  (Variables|Default|SetCharacterBP _ascharacter_bp)
  (bind _returnvalue (Game|SpawnActorfromClass "/Game/Assets/Weapon/Dubinka/DubinkaBP.DubinkaBP_C" (Transformation|GetWorldTransform _mesh) "Undefined" 0 0))
  (bind _output_get (Variables|Default|SetDubinka _returnvalue))
  (Transformation|AttachComponentToComponent _output_get _mesh "Dubinka" "SnapToTarget" "SnapToTarget" "SnapToTarget" true))

(fn ConstructionScript)