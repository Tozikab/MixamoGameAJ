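; GameMode_BP is a game mode Blueprint meant to react to player death by showing a widget.
; On BeginPlay it checks the player Character_BP's CharacterIsDead flag once and, only if set, binds to its own OnDestroyed event.
; That handler creates NewWidgetBlueprint_2 and adds it to the viewport.
; Respawn logic that spawns and possesses a new character is unconnected, and the Respawn event is empty.
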(event Custom|OnDstr
  (params (DestroyedActor :type Actor%20Object%20Reference))
  (bind _returnvalue (UserInterface|CreateWidget "/Game/HUD/NewWidgetBlueprint_2.NewWidgetBlueprint_2_C"))
  (UserInterface|Viewport|AddtoViewport _returnvalue 0))

(event Custom|Respawn)

(event EventBeginPlay
  (bind _ascharacter_bp (Utilities|Casting|CastToCharacter_BP (Game|GetPlayerCharacter 0)))
  (if (Variables|/Game/Blueprints/Character/MainCharacter/Character_BP.Character_BP_C|GetCharacterIsDead _ascharacter_bp)
    (Game|BindEventtoOnDestroyed (delegate Custom|OnDstr))))

(fn ConstructionScript)