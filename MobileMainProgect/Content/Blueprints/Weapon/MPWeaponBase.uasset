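; MPWeaponBase is a base weapon Blueprint that outlines firing and reloading.
; Fire and StopFire are empty events, and the construction script does nothing.
; Reload branches on AbleToReload, which returns true when AmmoInBag is above zero and AmmoCount differs from AmmoMax.
; The branch has no follow-up logic, so this graph never changes ammo.
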(event Custom|Fire)

(event Custom|Reload
  (if (CallFunction|AbletoReload)
    _))

(event Custom|StopFire)

(fn ConstructionScript)

(fn AbletoReload
  (if (and (> (Variables|Default|GetAmmoInBag) 0) (!= (Variables|Default|GetAmmoCount) (Variables|Default|GetAmmoMax)))
    (return true)
    (else
      (return false))))